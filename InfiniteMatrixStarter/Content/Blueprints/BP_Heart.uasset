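; BP_Heart is a spinning heart pickup that restores one point of player health.
; Overlapping its CONSUME_HEART component raises BP_Player's CurrentHealth, capped at MaxHealth, without destroying the heart.
; Tick rotates the heart and destroys it once the player pawn is more than 50 units past it along world X.
; A RemoveHeart function, not called within this Blueprint, removes HitHeartWidget and prints a debug string.
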(event `self.CONSUME_HEART.OnComponentBeginOverlap`
  (params (OverlappedComponent :type "PrimitiveComponent Object Reference") (OtherActor :type "Actor Object Reference") (OtherComp :type "PrimitiveComponent Object Reference") (OtherBodyIndex :type Integer) (bFromSweep :type Boolean) (SweepResult :type "HitResult Structure (by ref)"))
  (bind _asbp_player (cast `/Game/InfiniteMatrix/Blueprints/BP_Player` OtherActor))
  (set `/Game/InfiniteMatrix/Blueprints/BP_Player.CurrentHealth` (`KismetMathLibrary.Min` (`/Game/InfiniteMatrix/Blueprints/BP_Player.MaxHealth` _asbp_player) (+ (`/Game/InfiniteMatrix/Blueprints/BP_Player.CurrentHealth` _asbp_player) 1)) _asbp_player))

(event `self.ReceiveTick`
  (params (DeltaSeconds :type "Float (single-precision)"))
  (bind _returnvalue_x (`KismetMathLibrary.BreakVector` (`self.K2_GetActorLocation`)))
  (bind _returnvalue_x_2 (`KismetMathLibrary.BreakVector` (`self.K2_GetActorLocation` (`GameplayStatics.GetPlayerPawn` 0))))
  (`SceneComponent.K2_AddLocalRotation` (`self.CONSUME_HEART`) (`KismetMathLibrary.MakeRotator` 0.0 0.0 (`self.RotationSpeed`)) false false)
  (if (> _returnvalue_x_2 (+ _returnvalue_x 50.0))
    (`self.K2_DestroyActor`)))

(fn `RemoveHeart`
  (`Widget.RemoveFromParent` (`self.HitHeartWidget`))
  (`KismetSystemLibrary.PrintString` "Helasdlo"))

(fn `UserConstructionScript`)