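; BP_Damage is a spinning hazard actor that costs the player health on contact and can be destroyed for score.
; Tick rotates the damage component and destroys the actor once the player pawn is more than 50 units past it along X.
; On overlap, BP_Player loses one health, guarded to happen only once, and is marked dead with a restart display at zero.
; Overlap with BP_Sphere destroys the hazard and increments the player's Score.
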(event `self.ReceiveTick`
  (params (DeltaSeconds :type "Float (single-precision)"))
  (bind _returnvalue_x (`KismetMathLibrary.BreakVector` (`self.K2_GetActorLocation`)))
  (bind _returnvalue_x_2 (`KismetMathLibrary.BreakVector` (`self.K2_GetActorLocation` (`GameplayStatics.GetPlayerPawn` 0))))
  (`SceneComponent.K2_AddLocalRotation` (`self.CONSUME_DAMAGE`) (`KismetMathLibrary.MakeRotator` 0.0 0.0 (`self.RotationSpeed`)) false false)
  (if (> _returnvalue_x_2 (+ _returnvalue_x 50.0))
    (`self.K2_DestroyActor`)))

(event `self.CONSUME_DAMAGE.OnComponentBeginOverlap`
  (params (OverlappedComponent :type "PrimitiveComponent Object Reference") (OtherActor :type "Actor Object Reference") (OtherComp :type "PrimitiveComponent Object Reference") (OtherBodyIndex :type Integer) (bFromSweep :type Boolean) (SweepResult :type "HitResult Structure (by ref)"))
  (bind _asbp_player (cast `/Game/InfiniteMatrix/Blueprints/BP_Player` OtherActor)
    (:`then`
      (if (== (`self.Once`) false)
        (set `self.Once` true)
        (bind _result (`/Engine/EditorBlueprintResources/StandardMacros.DecrementInt` (`/Game/InfiniteMatrix/Blueprints/BP_Player.CurrentHealth` _asbp_player))
          (:`  `
            (if (<= _result 0)
              (set `/Game/InfiniteMatrix/Blueprints/BP_Player.IsDead` true _asbp_player)
              (`/Game/InfiniteMatrix/Blueprints/BP_Player.DisplayRestart` _asbp_player))))))
    (:`CastFailed`
      (cast `/Game/Blueprints/BP_Sphere` OtherActor)
      (`self.K2_DestroyActor`)
      (bind _asbp_player_2 (cast `/Game/InfiniteMatrix/Blueprints/BP_Player` (`GameplayStatics.GetPlayerPawn` 0)))
      (set `/Game/InfiniteMatrix/Blueprints/BP_Player.Score` (+ (`/Game/InfiniteMatrix/Blueprints/BP_Player.Score` _asbp_player_2) 1) _asbp_player_2))))

(fn `UserConstructionScript`)