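; BP_HeartSpawner spawns BP_Heart pickups ahead of the procedurally spawned tunnel.
; SpawnHeartRandom, on a 30% roll, finds the first BP_TunnelSpawner and offsets its NewestTunnel SpawnPoint by a random forward distance and lateral and vertical jitter.
; SpawnHeart spawns the heart at that location and keeps a reference to it.
; The event graph is empty, so both functions rely on outside callers.
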(event `self.ReceiveBeginPlay`)

(fn `Spawn Heart`
  (params (Location :type "Vector Structure"))
  (bind _returnvalue (`|SpawnActorFromClass` "/Game/Blueprints/BP_Heart.BP_Heart_C" (`KismetMathLibrary.MakeTransform` Location) "Undefined" "OverrideRootScale" null null))
  (set `self.Heart` _returnvalue))

(fn `SpawnHeartRandom`
  (locals (NewLocalVar_0 :type "Array of /Game/InfiniteMatrix/Blueprints/BP_TunnelSpawner Object Reference"))
  (bind _returnvalue (`KismetMathLibrary.RandomFloatInRange` -250.0 250.0))
  (bind _outactors (`GameplayStatics.GetAllActorsOfClass` "/Game/InfiniteMatrix/Blueprints/BP_TunnelSpawner.BP_TunnelSpawner_C"))
  (if (`KismetMathLibrary.RandomBoolWithWeight` 0.3)
    (`self.Spawn Heart` (+ (`SceneComponent.K2_GetComponentLocation` (`/Game/InfiniteMatrix/Blueprints/BP_Tunnel.SpawnPoint` (`/Game/InfiniteMatrix/Blueprints/BP_TunnelSpawner.NewestTunnel` (`|GetArrayItem` _outactors)))) (`KismetMathLibrary.MakeVector` (`KismetMathLibrary.RandomFloatInRange` 300.0 2000.0) _returnvalue _returnvalue)))))

(fn `UserConstructionScript`)